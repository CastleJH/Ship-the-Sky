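; Player controller that drives the owning-island tile UI in what appears to be a tile-based island strategy game.
; Events cast IslandTileUI to show or collapse its canvas and switch the building panel between closed, construction, barracks and shipyard views by index.
; GetTileResourcesUIHolder maps X/Y coordinates to a flattened grid of resource UI holders, dividing by HolderSize so each holder covers a block.
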(event EventBeginPlay)

(event EventTick
  (params (DeltaSeconds :type Float%20%28single-precision%29)))

(event EventOpenOwningIslandConstructionPanel
  (bind _aswbp_owning_island_tile_ui (Utilities|Casting|CastToWBP_OwningIslandTileUI (Variables|Default|GetIslandTileUI)))
  (Default|SetBuildingPanelActiveWidgetIndex _aswbp_owning_island_tile_ui 1))

(event EventOpenOwningIslandBarracksPanel
  (bind _aswbp_owning_island_tile_ui (Utilities|Casting|CastToWBP_OwningIslandTileUI (Variables|Default|GetIslandTileUI)))
  (Default|SetBuildingPanelActiveWidgetIndex _aswbp_owning_island_tile_ui 2))

(event EventOpenOwningIslandShipyardPanel
  (bind _aswbp_owning_island_tile_ui (Utilities|Casting|CastToWBP_OwningIslandTileUI (Variables|Default|GetIslandTileUI)))
  (Default|SetBuildingPanelActiveWidgetIndex _aswbp_owning_island_tile_ui 3))

(event EventCloseAllOwningIslandPanel
  (bind _aswbp_owning_island_tile_ui (Utilities|Casting|CastToWBP_OwningIslandTileUI (Variables|Default|GetIslandTileUI)))
  (Default|SetCanvasVisibility _aswbp_owning_island_tile_ui "Collapsed"))

(event EventOpenOwningIslandPanel
  (bind _aswbp_owning_island_tile_ui (Utilities|Casting|CastToWBP_OwningIslandTileUI (Variables|Default|GetIslandTileUI)))
  (Default|SetCanvasVisibility _aswbp_owning_island_tile_ui "Visible"))

(event EventCloseOwningIslandBuildingPanel
  (bind _aswbp_owning_island_tile_ui (Utilities|Casting|CastToWBP_OwningIslandTileUI (Variables|Default|GetIslandTileUI)))
  (Default|SetBuildingPanelActiveWidgetIndex _aswbp_owning_island_tile_ui))

(fn ConstructionScript)

(fn GetTileResourcesUIHolder
  (params (X :type Integer) (Y :type Integer))
  (bind _holdersize (Variables|Default|GetHolderSize))
  (bind _astile_resources_uiholder (Utilities|Casting|CastToBP_TileResourcesUIHolder (Utilities|Array|Get(acopy) (Variables|Default|GetTileResourcesUIHolders) (+ (* (/ X _holdersize) (Variables|Default|GetTileResourcesUIHolderCol)) (/ Y _holdersize)))))
  (return _astile_resources_uiholder))