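; Forest island tile actor that shows its resources on a widget component attached to the tile.
; On the resource UI update event, it reads its Resources map and fills the widget's three slots, using icons from the player controller's ResourcesTexture indexed by resource key.
; The first two slots show their map values, while the third always shows zero.
; An older path creating the UI through a controller-provided holder is left unconnected.
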(event EventBeginPlay)

(event Collision|EventActorBeginOverlap
  (params (OtherActor :type Actor%20Object%20Reference)))

(event EventTick
  (params (DeltaSeconds :type Float%20%28single-precision%29)))

(event EventOnUpdateTileResourcesUI
  (CallFunction|UpdateTileResourcesUI))

(fn ConstructionScript)

(fn UpdateTileResourcesUI
  (bind _resources (Variables|Default|GetResources))
  (bind _asbp_stsplayer_controller (Utilities|Casting|CastToBP_STSPlayerController (Game|GetPlayerController 0)))
  (bind _keys (Utilities|Map|Keys _resources))
  (bind _values (Utilities|Map|Values _resources))
  (bind _aswbp_tile_resources_ui (Utilities|Casting|CastToWBP_TileResourcesUI (UserInterface|GetWidget (Variables|Default|GetResourcesWidgetComp))))
  (Default|Set1stTileResourceInfo _aswbp_tile_resources_ui (Utilities|Array|Get(acopy) (Variables|/Script/ShipTheSky.STSPlayerController|GetResourcesTexture _asbp_stsplayer_controller) (Math|Conversions|ToInteger(Byte) (Utilities|Array|Get(acopy) _keys))) (Utilities|Array|Get(acopy) _values))
  (Default|Set2ndTileResourceInfo _aswbp_tile_resources_ui (Utilities|Array|Get(acopy) (Variables|/Script/ShipTheSky.STSPlayerController|GetResourcesTexture _asbp_stsplayer_controller) (Math|Conversions|ToInteger(Byte) (Utilities|Array|Get(acopy) _keys 1))) (Utilities|Array|Get(acopy) _values 1))
  (Default|Set3rdTileResourceInfo _aswbp_tile_resources_ui (Utilities|Array|Get(acopy) (Variables|/Script/ShipTheSky.STSPlayerController|GetResourcesTexture _asbp_stsplayer_controller) (Math|Conversions|ToInteger(Byte) (Utilities|Array|Get(acopy) _keys 2)))))